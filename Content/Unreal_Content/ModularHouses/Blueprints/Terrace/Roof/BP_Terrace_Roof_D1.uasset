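; Modular terrace roof piece for houses, built in the construction script with an adjustable width.
; A spline mesh (Side) stretches out to Width, with tangents derived from the start and end transforms, and a static mesh is added at each end.
; All three share a configurable material, while dynamic instances on two Side slots scale U tiling with width.
; Two flags hide the end rails and their shadows.
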(fn ConstructionScript
  (bind _width (Variables|Default|GetWidth))
  (bind _width_2 (Variables|Default|GetWidth))
  (bind _end (Variables|Default|GetEnd))
  (bind _end_transform (Variables|Default|GetEnd%20transform))
  (bind _start_transform (Variables|Default|GetStart%20transform))
  (bind _returnvalue (- _width_2 1.2e+02))
  (bind (_location _rotation _scale) (Math|Transform|BreakTransform _start_transform))
  (bind (_x _y _z) (Math|Vector|BreakVector _end))
  (bind (_location_2 _rotation_2 _scale_2) (Math|Transform|BreakTransform _end_transform))
  (bind _returnvalue_2 (Math|Vector|MakeVector _width _y _z))
  (bind _returnvalue_3 (- _location _location_2))
  (bind _returnvalue_4 (* _returnvalue 0.00625))
  (bind _returnvalue_5 (Math|Vector|VectorLength _returnvalue_3))
  (bind _returnvalue_6 (+ _returnvalue_4 1.0))
  (SplineMesh|SetStartandEnd (Variables|Default|GetSide) _location (* (* (Math|Vector|GetForwardVector _rotation) _scale) _returnvalue_5) _returnvalue_2 (* (* (Math|Vector|GetForwardVector _rotation_2) _scale_2) _returnvalue_5) true :!class /Script/Engine.SplineMeshComponent)
  (bind _returnvalue_7 (AddComponent|AddStaticMeshComponent false _start_transform))
  (bind _returnvalue_8 (AddComponent|AddStaticMeshComponent false (Math|Conversions|ToTransform(Vector) _returnvalue_2)))
  (Rendering|Material|SetMaterial _returnvalue_8 0 (Variables|Default|GetMaterial_1))
  (bind _returnvalue_9 (Rendering|Material|CreateDynamicMaterialInstance (Variables|Default|GetSide) 0 (Variables|Default|GetMaterial_1) "None" :!class /Script/Engine.PrimitiveComponent))
  (Rendering|Material|SetScalarParameterValue _returnvalue_9 "Tile_U" _returnvalue_6 :!class /Script/Engine.MaterialInstanceDynamic)
  (bind _returnvalue_10 (Rendering|Material|CreateDynamicMaterialInstance (Variables|Default|GetSide) 2 "/Game/Unreal_Content/ModularHouses/Materials/Generic/M_Plastic_Line_A_Inst.M_Plastic_Line_A_Inst" "None" :!class /Script/Engine.PrimitiveComponent))
  (Rendering|Material|SetScalarParameterValue _returnvalue_10 "Tile_U" _returnvalue_6 :!class /Script/Engine.MaterialInstanceDynamic)
  (if (Variables|Default|GetHide%20Rail%202)
    (Rendering|SetVisibility _returnvalue_8 false false)
    (Rendering|SetCastShadow _returnvalue_8 false))
  (if (Variables|Default|GetHide%20Rail_1)
    (Rendering|SetVisibility _returnvalue_7 false false)
    (Rendering|SetCastShadow _returnvalue_7 false)))