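; Character Blueprint that switches its mesh between numbered poses through a transition Anim Blueprint.
; ChangePose1 prints CurrInt and maps values 0-7 to NewPose for ChangePose.
; ChangePose records last and current pose, swaps the mesh to ABP_Transitions, then after a one-second lockout sets FinalTransition.
; Higher-pose selection, next/previous stepping and the per-pose Anim Blueprint switch are unwired, and FuncFinalPose is empty.
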(event Custom|ChangePose
  (bind _newpose (Variables|Default|GetNewPose))
  ;[0.3338 0.7006 1 1 35] ChangePose
  (if (and (!= _newpose (Variables|Default|GetPoseNumber)) (Variables|Default|GetCanChange))
    (Variables|Default|SetCanChange false)
    (Variables|Default|SetLastPose (Variables|Default|GetPoseNumber))
    (Variables|Default|SetPoseNumber _newpose)
    (Class|SkeletalMeshComponent|SetAnimClass (Variables|Character|GetMesh) "/Game/Unreal_Content/PoseAnimations/AimationBlueprints/ABP_Transitions.ABP_Transitions_C")
    (Utilities|FlowControl|Delay 1.0)
    (Variables|Default|SetCanChange true)
    (Variables|Default|SetFinalTransition true)))

(event Custom|ChangePose1
  (bind _currint (Variables|Default|GetCurrInt))
  (Development|PrintString (Utilities|String|ToString(Integer) _currint))
  (switch int _currint
    (:0
      ;[1 0.3708 0.4405 1 35] ChangePoseInput
      (Variables|Default|SetNewPose 0)
      (CallFunction|ChangePose))
    (:1
      (Variables|Default|SetNewPose 1)
      (CallFunction|ChangePose))
    (:2
      (Variables|Default|SetNewPose 2)
      (CallFunction|ChangePose))
    (:3
      (Variables|Default|SetNewPose 3)
      (CallFunction|ChangePose))
    (:4
      (Variables|Default|SetNewPose 4)
      (CallFunction|ChangePose))
    (:5
      (Variables|Default|SetNewPose 5)
      (CallFunction|ChangePose))
    (:6
      (Variables|Default|SetNewPose 6)
      (CallFunction|ChangePose))
    (:7
      (Variables|Default|SetNewPose 7)
      (CallFunction|ChangePose))))

(fn ConstructionScript)

(fn FuncFinalPose)