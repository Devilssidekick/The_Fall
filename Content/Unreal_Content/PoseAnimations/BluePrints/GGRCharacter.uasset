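; GGRCharacter is a character Blueprint that switches between numbered poses through number keys, letter keys and PageUp/PageDown stepping.
; Each key sets NewPose and calls ChangePose, which records the previous and new pose and swaps the mesh to ABP_Transitions.
; A CanChange gate blocks input during a one-second delay, then FinalTransition is set.
; The per-pose AnimBP switch in Func_FinalPose is disconnected and never runs.
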(event Custom|ChangePose
  (bind _newpose (Variables|Default|GetNewPose))
  ;[0.3338 0.7006 1 1 35] ChangePose
  (if (and (!= _newpose (Variables|Default|GetPoseNumber)) (Variables|Default|GetCanChange))
    (Variables|Default|SetCanChange false)
    (Variables|Default|SetLastPose (Variables|Default|GetPoseNumber))
    (Variables|Default|SetPoseNumber _newpose)
    (Class|SkeletalMeshComponent|SetAnimClass (Variables|Character|GetMesh) "/Game/Unreal_Content/PoseAnimations/AimationBlueprints/ABP_Transitions.ABP_Transitions_C")
    (Utilities|FlowControl|Delay 1.0)
    (Variables|Default|SetCanChange true)
    (Variables|Default|SetFinalTransition true)))

(event Input|KeyboardEvents|0
  (params (Key :type Key%20Structure :default "None"))
  ;[1 0.3708 0.4405 1 35] ChangePoseInput
  (:Pressed
    (Variables|Default|SetNewPose 0)
    (CallFunction|ChangePose)))

(event Input|KeyboardEvents|1
  (params (Key :type Key%20Structure :default "None"))
  ;[1 0.3708 0.4405 1 35] ChangePoseInput
  (:Pressed
    (Variables|Default|SetNewPose 1)
    (CallFunction|ChangePose)))

(event Input|KeyboardEvents|P
  (params (Key :type Key%20Structure :default "None"))
  ;[1 0.3708 0.4405 1 35] ChangePoseInput
  (:Pressed
    (Variables|Default|SetNewPose 14)
    (CallFunction|ChangePose)))

(event Input|KeyboardEvents|Y
  (params (Key :type Key%20Structure :default "None"))
  ;[1 0.3708 0.4405 1 35] ChangePoseInput
  (:Pressed
    (Variables|Default|SetNewPose 10)
    (CallFunction|ChangePose)))

(event Input|KeyboardEvents|U
  (params (Key :type Key%20Structure :default "None"))
  ;[1 0.3708 0.4405 1 35] ChangePoseInput
  (:Pressed
    (Variables|Default|SetNewPose 11)
    (CallFunction|ChangePose)))

(event Input|KeyboardEvents|I
  (params (Key :type Key%20Structure :default "None"))
  ;[1 0.3708 0.4405 1 35] ChangePoseInput
  (:Pressed
    (Variables|Default|SetNewPose 12)
    (CallFunction|ChangePose)))

(event Input|KeyboardEvents|O
  (params (Key :type Key%20Structure :default "None"))
  ;[1 0.3708 0.4405 1 35] ChangePoseInput
  (:Pressed
    (Variables|Default|SetNewPose 13)
    (CallFunction|ChangePose)))

(event Input|KeyboardEvents|PageUp
  (params (Key :type Key%20Structure :default "None"))
  ;[1 0.3708 0.4405 1 35] ChangePoseInput
  (:Pressed
    (Variables|Default|SetNewPose (+ (Variables|Default|GetPoseNumber) 1))
    (CallFunction|ChangePose)))

(event Input|KeyboardEvents|PageDown
  (params (Key :type Key%20Structure :default "None"))
  ;[1 0.3708 0.4405 1 35] ChangePoseInput
  (:Pressed
    (Variables|Default|SetNewPose (- (Variables|Default|GetPoseNumber) 1))
    (CallFunction|ChangePose)))

(event Input|KeyboardEvents|2
  (params (Key :type Key%20Structure :default "None"))
  ;[1 0.3708 0.4405 1 35] ChangePoseInput
  (:Pressed
    (Variables|Default|SetNewPose 2)
    (CallFunction|ChangePose)))

(event Input|KeyboardEvents|3
  (params (Key :type Key%20Structure :default "None"))
  ;[1 0.3708 0.4405 1 35] ChangePoseInput
  (:Pressed
    (Variables|Default|SetNewPose 3)
    (CallFunction|ChangePose)))

(event Input|KeyboardEvents|4
  (params (Key :type Key%20Structure :default "None"))
  ;[1 0.3708 0.4405 1 35] ChangePoseInput
  (:Pressed
    (Variables|Default|SetNewPose 4)
    (CallFunction|ChangePose)))

(event Input|KeyboardEvents|5
  (params (Key :type Key%20Structure :default "None"))
  ;[1 0.3708 0.4405 1 35] ChangePoseInput
  (:Pressed
    (Variables|Default|SetNewPose 5)
    (CallFunction|ChangePose)))

(event Input|KeyboardEvents|6
  (params (Key :type Key%20Structure :default "None"))
  ;[1 0.3708 0.4405 1 35] ChangePoseInput
  (:Pressed
    (Variables|Default|SetNewPose 6)
    (CallFunction|ChangePose)))

(event Input|KeyboardEvents|7
  (params (Key :type Key%20Structure :default "None"))
  ;[1 0.3708 0.4405 1 35] ChangePoseInput
  (:Pressed
    (Variables|Default|SetNewPose 7)
    (CallFunction|ChangePose)))

(event Input|KeyboardEvents|8
  (params (Key :type Key%20Structure :default "None"))
  ;[1 0.3708 0.4405 1 35] ChangePoseInput
  (:Pressed
    (Variables|Default|SetNewPose 8)
    (CallFunction|ChangePose)))

(event Input|KeyboardEvents|9
  (params (Key :type Key%20Structure :default "None"))
  ;[1 0.3708 0.4405 1 35] ChangePoseInput
  (:Pressed
    (Variables|Default|SetNewPose 9)
    (CallFunction|ChangePose)))

(fn ConstructionScript)

(fn FuncFinalPose)