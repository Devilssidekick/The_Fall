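; BP_FotoTeleport is an actor that teleports the first-person player to a target position from a trigger collider.
; BeginPlay caches the player and activates the teleporter; overlapping the collider sets an inside flag.
; While inside and active, Tick polls the player's IisPresed flag, then moves them to TeleportPos's Rrr component.
; The inside flag clears only on teleport, and a note marks the logic as provisional, to move into the player.
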(event OnComponentBeginOverlap(Collider)
  (params (OverlappedComponent :type Primitive%20Component%20Object%20Reference) (OtherActor :type Actor%20Object%20Reference) (OtherComp :type Primitive%20Component%20Object%20Reference) (OtherBodyIndex :type Integer) (bFromSweep :type Boolean) (SweepResult :type Hit%20Result%20Structure%20%28by%20ref%29))
  ;[1 1 1] Ja moin das muss halt später über den PLayer passieren, so ist das natürlich ein bsischen dumm .. und später dann auch checken, ob object in view sit
  (Utilities|Casting|CastToFirstPersonCharacter OtherActor)
  (Development|PrintString "Ok")
  (Variables|Default|SetIsInside true))

(event Custom|Teleprt
  (bind _player (Variables|Default|GetPlayer))
  ;[1 1 1] Teleport Player to New Position if Active
  (if (Variables|Default|GetIsInside)
    (if (Variables|/Game/Unreal_Content/FirstPersonBP/Blueprints/FirstPersonCharacter.FirstPersonCharacter_C|GetIisPresed _player)
      (Transformation|SetActorLocation _player (Transformation|GetWorldLocation (Variables|/Game/Actors/TeleportPos.TeleportPos_C|Getrrr (Variables|Default|GetTeleportPos))) false false)
      (Variables|Default|SetIsInside false))))

(event EventBeginPlay
  ;[1 1 1] Set Player
  (bind _asfirst_person_character (Utilities|Casting|CastToFirstPersonCharacter (Game|Player|GetPlayerPawn 0)))
  (Variables|Default|SetPlayer _asfirst_person_character)
  (Variables|Default|SetIsActive true))

(event Collision|EventActorBeginOverlap
  (params (OtherActor :type Actor%20Object%20Reference)))

(event EventTick
  (params (DeltaSeconds :type Float%20%28single-precision%29))
  (if (Variables|Default|GetIsInside)
    (if (Variables|Default|GetIsActive)
      (CallFunction|Teleprt))))

(fn ConstructionScript)